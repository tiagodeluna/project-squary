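; Door actor for Squary that acts as the exit to the next level.
; OpenDoor swaps the Cube material to grey and sets IsOpen, and runs on BeginPlay when the door already starts open.
; ChangeLevel loads the level named in NextLevel only while the door is open.
; The opening animation is still a TODO, so the material swap is the only visual change.
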(event `self.ReceiveBeginPlay`
  ;[1 1 1] Open Door When Level Is Open
  (if (`self.IsOpen`)
    (`self.OpenDoor`)))

(event `OpenDoor`
  ;[1 1 1] Custom Event: Open Door
  ;;[1 1 1] TODO: There will be an animation to apply
  (`PrimitiveComponent.SetMaterial` (`self.Cube`) 0 "/Game/Squary/Materials/Grey.Grey")
  (set `self.IsOpen` true))

(event `ChangeLevel`
  ;[1 1 1] Custom Event: Change Level
  (if (`self.IsOpen`)
    (`GameplayStatics.OpenLevel` (`self.NextLevel`))))

(fn `UserConstructionScript`)